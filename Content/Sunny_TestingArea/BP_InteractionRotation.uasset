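; Interactable actor that swings a mesh open and closed by rotating it, with an optional lock requiring a tagged item.
; Interact toggles based on the mesh's current relative rotation, playing or reversing a speed-scaled timeline that lerps to OpenDistance around the chosen, flippable axis.
; The timeline also sets IsTimelinePlaying on the player character while running.
; The construction script applies QuickNewMesh and rotates an arrow to preview the open rotation.
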(event `self.ReceiveBeginPlay`
  (bind _asthird_person_character (cast `/Game/ThirdPersonBP/Blueprints/ThirdPersonCharacter` (`GameplayStatics.GetPlayerCharacter` 0)))
  (set `self.PlayerRef` _asthird_person_character)
  (set `self.MeshesToAffect` (`|MakeArray` (`self.StaticMesh1`) :!type "SceneComponent Object Reference"))
  (`TimelineComponent.SetPlayRate` (`self.Open`) (`self.Speed`)))

(event `/Game/Sunny_TestingArea/Interactables/BPI_Interact.Interact`
  (params (InteractingComponent :type "PrimitiveComponent Object Reference (by ref)"))
  ;[1 1 1] Check if the drawer is opened or close (if the drawer's location is equal to the location+distance then the drawer is open so close it)
  (for _array_element (`self.MeshesToAffect`)
    (if (== _array_element InteractingComponent)
      (set `self.InteractingObj` InteractingComponent)))
  (if (`self.Locked?`)
    (if (`/Game/Sunny_TestingArea/Interactables/BPFL_Interact.CheckHasRequiredItem?` (`self.Tags`))
      (if (!= (`SceneComponent.RelativeRotation` (`self.InteractingObj`)) (struct)) :!label _label
        (`self.CloseDrawer`)
        (else
          (`self.OpenDrawer`))))
    (else
      (goto _label))))

(event `OpenDrawer`
  (bind _opendistance (`self.OpenDistance`))
  (bind _playerref (`self.PlayerRef`))
  (bind _returnvalue (select `bool` (`self.FlipOpeningDirection?`) :`false` _opendistance :`true` (* _opendistance -1.0)))
  ;[1 1 1] Just a basic timeline that opens and closes the drawer using a lerp
  (`TimelineComponent.SetPlaybackPosition` (`self.Open`) 0.0 false true)
  (bind (_direction _alpha) (`Timeline|Open` :!label _label_2)
    (:`Update`
      (set `/Game/ThirdPersonBP/Blueprints/ThirdPersonCharacter.bIsTimelinePlaying?` true _playerref)
      (`SceneComponent.K2_SetRelativeRotation` (`self.InteractingObj`) (`KismetMathLibrary.RLerp` (`KismetMathLibrary.MakeRotator` 0.0) (select `/Game/Sunny_TestingArea/E_Direction` (`self.Direction`) :`NewEnumerator0` (`KismetMathLibrary.MakeRotator` 0.0 _returnvalue) :`NewEnumerator1` (`KismetMathLibrary.MakeRotator` _returnvalue) :`NewEnumerator2` (`KismetMathLibrary.MakeRotator` 0.0 0.0 _returnvalue)) _alpha) false false))
    (:`Finished`
      (set `/Game/ThirdPersonBP/Blueprints/ThirdPersonCharacter.bIsTimelinePlaying?` false _playerref))))

(event `CloseDrawer`
  ;[1 1 1] Just a basic timeline that opens and closes the drawer using a lerp
  (`TimelineComponent.SetPlaybackPosition` (`self.Open`) 1.0 false true)
  (goto _label_2 :!via `Reverse`))

(fn `UserConstructionScript`
  (bind _opendistance (`self.OpenDistance`))
  (bind _returnvalue (select `bool` (`self.FlipOpeningDirection?`) :`false` _opendistance :`true` (* _opendistance -1.0)))
  (`StaticMeshComponent.SetStaticMesh` (`self.StaticMesh1`) (`self.QuickNewMesh`))
  (`SceneComponent.K2_SetRelativeRotation` (`self.Arrow`) (select `/Game/Sunny_TestingArea/E_Direction` (`self.Direction`) :`NewEnumerator0` (`KismetMathLibrary.MakeRotator` 0.0 _returnvalue) :`NewEnumerator1` (`KismetMathLibrary.MakeRotator` _returnvalue) :`NewEnumerator2` (`KismetMathLibrary.MakeRotator` 0.0 0.0 _returnvalue)) false false))