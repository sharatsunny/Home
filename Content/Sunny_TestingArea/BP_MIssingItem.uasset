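; BP_MIssingItem is a placeholder for a missing object that the player restores with a matching inventory item.
; The construction script gives the chosen mesh "missing" and outline materials and fits a trigger sphere to its bounds.
; Overlap registers it with ThirdPersonCharacter and fades the outline through a timeline.
; Interact compares the previewed item's name to actor tags, restoring the material and consuming the item, or playing random subtitles on mismatch.
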(event `self.ReceiveBeginPlay`
  (bind _asthird_person_character (cast `/Game/ThirdPersonBP/Blueprints/ThirdPersonCharacter` (`GameplayStatics.GetPlayerCharacter` 0)))
  (set `self.PlayerRef` _asthird_person_character))

(event `self.Sphere.OnComponentBeginOverlap`
  (params (OverlappedComponent :type "PrimitiveComponent Object Reference") (OtherActor :type "Actor Object Reference") (OtherComp :type "PrimitiveComponent Object Reference") (OtherBodyIndex :type Integer) (bFromSweep :type Boolean) (SweepResult :type "HitResult Structure (by ref)"))
  (bind _asthird_person_character (cast `/Game/ThirdPersonBP/Blueprints/ThirdPersonCharacter` OtherActor))
  (bind _output_get (set `self.PlayerRef` _asthird_person_character))
  (set `/Game/ThirdPersonBP/Blueprints/ThirdPersonCharacter.MissingObjBPInRange` self _output_get)
  (set `self.bIsOverlapping?` true)
  (bind (_direction _alpha) (`Timeline|Update` :!label _label)
    (:`Update`
      (`MaterialInstanceDynamic.SetScalarParameterValue` (`self.OutlineMaterialRef`) "BlendAmount" (`KismetMathLibrary.Lerp` 0.0 (`self.BlendAmount`) _alpha)))))

(event `self.Sphere.OnComponentEndOverlap`
  (params (OverlappedComponent :type "PrimitiveComponent Object Reference") (OtherActor :type "Actor Object Reference") (OtherComp :type "PrimitiveComponent Object Reference") (OtherBodyIndex :type Integer))
  (bind _asthird_person_character (cast `/Game/ThirdPersonBP/Blueprints/ThirdPersonCharacter` OtherActor))
  (bind _output_get (set `self.PlayerRef` _asthird_person_character))
  (set `/Game/ThirdPersonBP/Blueprints/ThirdPersonCharacter.MissingObjBPInRange` null _output_get)
  (set `self.bIsOverlapping?` false)
  (goto _label :!via `Reverse`))

(event `/Game/Sunny_TestingArea/Interactables/BPI_Interact.Interact`
  (params (InteractingComponent :type "PrimitiveComponent Object Reference (by ref)"))
  (bind _returnvalue (`GameplayStatics.GetPlayerController` 0))
  (bind _playerref (`self.PlayerRef`))
  (bind _subtitles (`self.Subtitles`))
  (bind _playerref_2 (`self.PlayerRef`))
  (bind _returnvalue_2 (`KismetMathLibrary.RandomInteger` (- (`BlueprintMapLibrary.Map_Length` _subtitles) 1)))
  (if (`self.bIsOverlapping?`)
    (for _array_element (`self.Tags`)
      (if (== _array_element (`KismetStringLibrary.Conv_StringToName` (`KismetTextLibrary.Conv_TextToString` (`TextBlock.GetText` (`/Game/UMG/ItemInspection/UI_ItemPreview.ItemName` (`/Game/UMG/UMG_PlayerHUD.UI_ItemPreview_Current` (`/Game/ThirdPersonBP/Blueprints/ThirdPersonCharacter.UI_PlayerHUD` (`self.PlayerRef`))))))))
        (set `self.ItemMatched` true)
        (`/Game/UMG/UMG_PlayerHUD.HideInventory` (`/Game/ThirdPersonBP/Blueprints/ThirdPersonCharacter.UI_PlayerHUD` _playerref))
        (set `/Game/ThirdPersonBP/Blueprints/ThirdPersonCharacter.bIsInInventory?` false _playerref)
        (set `PlayerController.bShowMouseCursor` false _returnvalue)
        (`WidgetBlueprintLibrary.SetInputMode_GameOnly` _returnvalue)
        (`PrimitiveComponent.SetMaterial` (`self.StaticMesh`) 0 (`self.DefaultMaterial`))
        (`SceneComponent.SetVisibility` (`self.SM_Outline`) false false)
        (`KismetArrayLibrary.Array_Remove` (`/Game/ThirdPersonBP/Blueprints/ThirdPersonCharacter.Inventory` (`self.PlayerRef`)) (`/Game/UMG/ItemInspection/UI_ItemPreview.Index` (`/Game/UMG/UMG_PlayerHUD.UI_ItemPreview_Current` (`/Game/ThirdPersonBP/Blueprints/ThirdPersonCharacter.UI_PlayerHUD` (`self.PlayerRef`)))))))
    (if (not (`self.ItemMatched`))
      (set `/Game/ThirdPersonBP/Blueprints/ThirdPersonCharacter.bIsSubsPlaying?` true _playerref_2)
      (bind _keys (`BlueprintMapLibrary.Map_Keys` _subtitles))
      (bind _values (`BlueprintMapLibrary.Map_Values` _subtitles))
      (bind _output (`|GetArrayItem` _values _returnvalue_2))
      (message `/Game/Sunny_TestingArea/Interactables/BPI_Subtitle.SetSubtitleManually` (`/Game/ThirdPersonBP/Blueprints/ThirdPersonCharacter.UI_PlayerHUD` _playerref_2) (`|MakeMap` (`|GetArrayItem` _keys _returnvalue_2) (select `bool` (`KismetSystemLibrary.IsValid` _output) :`true` _output)) (`self.AutoFadeAfterAudio?`) (`self.DelayBeforeFade`) (`self.DelayLines?`) (`self.DelayBetweenLines`)))))

(fn `UserConstructionScript`
  (bind _staticmesh (`self.StaticMesh`))
  (bind _sm_outline (`self.SM_Outline`))
  (bind _sphere (`self.Sphere`))
  (bind _newstaticmesh (`self.NewStaticMesh`))
  (bind (_origin _boxextent _sphereradius) (`KismetSystemLibrary.GetComponentBounds` (`self.StaticMesh`)))
  (`|ExecutionSequence`
    (:`then_0`
      (`StaticMeshComponent.SetStaticMesh` _staticmesh _newstaticmesh)
      (set `self.DefaultMaterial` (`StaticMesh.GetMaterial` _newstaticmesh 0))
      (bind _returnvalue (`PrimitiveComponent.CreateDynamicMaterialInstance` _staticmesh 0 "/Game/Sunny_TestingArea/MI_Missing.MI_Missing" "None"))
      (set `self.MaterialRef` _returnvalue)
      (`PrimitiveComponent.SetMaterial` _staticmesh 0 _returnvalue)
      (`SceneComponent.K2_SetRelativeLocation` _sphere (`KismetMathLibrary.InverseTransformLocation` (`SceneComponent.K2_GetComponentToWorld` (`self.DefaultSceneRoot`)) _origin) false false)
      (`SphereComponent.SetSphereRadius` _sphere (* _sphereradius (`self.CollisionRadiusMultiplier`)) true))
    (:`then_1`
      (`StaticMeshComponent.SetStaticMesh` (`self.SM_Outline`) _newstaticmesh)
      (bind _returnvalue_2 (`PrimitiveComponent.CreateDynamicMaterialInstance` _sm_outline 0 "/Game/Sunny_TestingArea/MI_MissingOutline.MI_MissingOutline" "None"))
      (set `self.OutlineMaterialRef` _returnvalue_2)
      (`PrimitiveComponent.SetMaterial` _sm_outline 0 _returnvalue_2))))