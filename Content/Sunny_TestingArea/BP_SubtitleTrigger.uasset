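; A trigger volume that shows configured manual subtitles on the HUD when the ThirdPersonCharacter enters its box.
; A DoOnce gate on begin overlap flags the character as playing subtitles and passes the text, fade and line-delay settings to UIPlayerHUD.
; On end overlap, the gate resets only if CanReplay is set and that character's subtitles are no longer playing.
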(event `self.Box.OnComponentBeginOverlap`
  (params (OverlappedComponent :type "PrimitiveComponent Object Reference") (OtherActor :type "Actor Object Reference") (OtherComp :type "PrimitiveComponent Object Reference") (OtherBodyIndex :type Integer) (bFromSweep :type Boolean) (SweepResult :type "HitResult Structure (by ref)"))
  (bind _asthird_person_character (cast `/Game/ThirdPersonBP/Blueprints/ThirdPersonCharacter` OtherActor))
  (`/Engine/EditorBlueprintResources/StandardMacros.DoOnce` false :!label _label
    (:`Completed`
      (set `/Game/ThirdPersonBP/Blueprints/ThirdPersonCharacter.bIsSubsPlaying?` true _asthird_person_character)
      (message `/Game/Sunny_TestingArea/Interactables/BPI_Subtitle.SetSubtitleManually` (`/Game/ThirdPersonBP/Blueprints/ThirdPersonCharacter.UI_PlayerHUD` _asthird_person_character) (`self.ManualSubtitles`) (`self.AutoFadeAfterAudio?`) (`self.DelayBeforeFade`) (`self.DelayLines?`) (`self.DelayBetweenLines`)))))

(event `self.Box.OnComponentEndOverlap`
  (params (OverlappedComponent :type "PrimitiveComponent Object Reference") (OtherActor :type "Actor Object Reference") (OtherComp :type "PrimitiveComponent Object Reference") (OtherBodyIndex :type Integer))
  (bind _asthird_person_character (cast `/Game/ThirdPersonBP/Blueprints/ThirdPersonCharacter` OtherActor))
  (if (and (`self.CanReplay?`) (not (`/Game/ThirdPersonBP/Blueprints/ThirdPersonCharacter.bIsSubsPlaying?` _asthird_person_character)))
    (goto _label :!via `Reset`)))

(fn `UserConstructionScript`)