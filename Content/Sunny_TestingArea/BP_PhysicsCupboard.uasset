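; BP_PhysicsCupboard is an interactable cupboard whose meshes the player swings with the mouse, optionally locked behind a required item.
; Interact matches the clicked component against four meshes, then enables physics and flags the player as physics-interacting.
; Horizontal mouse input yaws that mesh.
; DisablePhysics polls via a timeline until interaction ends near the default yaw, then snaps the mesh back and disables physics.
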(event `self.ReceiveBeginPlay`
  ;[1 1 1] Sets the default rotation and assigns all the meshes into an array
  (bind _asthird_person_character (cast `/Game/ThirdPersonBP/Blueprints/ThirdPersonCharacter` (`GameplayStatics.GetPlayerCharacter` 0)))
  (set `self.PlayerRef` _asthird_person_character)
  (set `self.MeshesToAffect` (`|MakeArray` (`self.StaticMesh1`) (`self.StaticMesh2`) (`self.StaticMesh3`) (`self.StaticMesh4`)))
  (set `self.DefaultRotation` (`SceneComponent.K2_GetComponentRotation` (`self.StaticMesh`))))

(event `/Game/Sunny_TestingArea/Interactables/BPI_Interact.Interact`
  (params (InteractingComponent :type "PrimitiveComponent Object Reference (by ref)"))
  ;[1 1 1] finds out which mesh fromt the array of meshes was clicked on, if the 2 meshes match then set it as a new variable that we can re-use then do the normal check for enabling physics
  (for _array_element (`self.MeshesToAffect`)
    (if (== _array_element InteractingComponent)
      (set `self.InteractingObj` _array_element)))
  (if (`self.Locked?`)
    (if (`/Game/Sunny_TestingArea/Interactables/BPFL_Interact.CheckHasRequiredItem?` (`self.Tags`))
      (set `/Game/ThirdPersonBP/Blueprints/ThirdPersonCharacter.bIsPhysicsInteraction?` true (`self.PlayerRef`) :!label _label)
      (`PrimitiveComponent.SetSimulatePhysics` (`self.InteractingObj`) true))
    (else
      (goto _label))))

(event `/Game/Sunny_TestingArea/Interactables/BPI_Interact.PhysicsInteraction`
  (params (XValue :type "Float (single-precision)") (YValue :type "Float (single-precision)"))
  ;[1 1 1] rotates the door based on the mouse's horizontal axis value
  (if (`self.Locked?`)
    (if (`/Game/Sunny_TestingArea/Interactables/BPFL_Interact.CheckHasRequiredItem?` (`self.Tags`))
      (`SceneComponent.K2_AddWorldRotation` (`self.InteractingObj`) (`KismetMathLibrary.MakeRotator` 0.0 0.0 (* (* XValue (`self.SpeedMultiplier`)) -1.0)) false false :!label _label_2))
    (else
      (goto _label_2))))

(event `/Game/Sunny_TestingArea/Interactables/BPI_Interact.DisablePhysics`
  (bind (_defaultrotation_roll _defaultrotation_pitch _defaultrotation_yaw) (`KismetMathLibrary.BreakRotator` (`self.DefaultRotation`)))
  (bind (_returnvalue_roll _returnvalue_pitch _returnvalue_yaw) (`KismetMathLibrary.BreakRotator` (`SceneComponent.K2_GetComponentRotation` (`self.InteractingObj`))))
  ;[1 1 1] this checks if the current object that we're rotating is close to the original rotation if so then just reset everything
  (if (and (not (`/Game/ThirdPersonBP/Blueprints/ThirdPersonCharacter.bIsPhysicsInteraction?` (`self.PlayerRef`))) (`KismetMathLibrary.NearlyEqual_FloatFloat` _returnvalue_yaw _defaultrotation_yaw 10.0)) :!label _label_3
    (`SceneComponent.K2_SetWorldRotation` (`self.InteractingObj`) (`self.DefaultRotation`) false false)
    (`PrimitiveComponent.SetSimulatePhysics` (`self.InteractingObj`) false)
    (`Timeline|Timeline_0` :!via `Stop` :!label _label_4
      (:`Update`
        (goto _label_3)))
    (else
      (goto _label_4))))

(fn `UserConstructionScript`)