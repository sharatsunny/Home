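; Interactable drawer unit with three drawer meshes that slide open and closed when the player interacts with them, optionally locked behind a required item.
; Interact matches the hit component to its drawer, checks the item by tags if locked, then toggles based on the drawer's current Y position.
; One shared timeline, played or reversed at a configurable speed, lerps the selected drawer and flags the player while it runs.
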(event `self.ReceiveBeginPlay`
  (bind _asthird_person_character (cast `/Game/ThirdPersonBP/Blueprints/ThirdPersonCharacter` (`GameplayStatics.GetPlayerCharacter` 0)))
  (set `self.PlayerRef` _asthird_person_character)
  (set `self.MeshesToAffect` (`|MakeArray` (`self.StaticMesh1`) (`self.StaticMesh2`) (`self.StaticMesh3`)))
  (`TimelineComponent.SetPlayRate` (`self.Open`) (`self.Speed`)))

(event `/Game/Sunny_TestingArea/Interactables/BPI_Interact.Interact`
  (params (InteractingComponent :type "PrimitiveComponent Object Reference (by ref)"))
  (bind (_relativelocation_x _relativelocation_y _relativelocation_z) (`KismetMathLibrary.BreakVector` (`SceneComponent.RelativeLocation` (`self.InteractingObj`))))
  ;[1 1 1] Enables the physics for selected obect
  (for _array_element (`self.MeshesToAffect`)
    (if (== _array_element InteractingComponent)
      (set `self.InteractingObj` _array_element)))
  (if (`self.Locked?`)
    (if (`/Game/Sunny_TestingArea/Interactables/BPFL_Interact.CheckHasRequiredItem?` (`self.Tags`))
      (if (== (`SceneComponent.RelativeLocation` (`self.InteractingObj`)) (`KismetMathLibrary.MakeVector` _relativelocation_x (`self.OpenDistance`) _relativelocation_z) :`ErrorTolerance` 1.0) :!label _label
        (`self.CloseDrawer`)
        (else
          (`self.OpenDrawer`))))
    (else
      (goto _label))))

(event `OpenDrawer`
  (bind _interactingobj (`self.InteractingObj`))
  (bind _playerref (`self.PlayerRef`))
  (bind (_relativelocation_x _relativelocation_y _relativelocation_z) (`KismetMathLibrary.BreakVector` (`SceneComponent.RelativeLocation` _interactingobj)))
  (`TimelineComponent.SetPlaybackPosition` (`self.Open`) 0.0 false true)
  (bind (_direction _alpha) (`Timeline|Open` :!label _label_2)
    (:`Update`
      (set `/Game/ThirdPersonBP/Blueprints/ThirdPersonCharacter.bIsTimelinePlaying?` true _playerref)
      (`SceneComponent.K2_SetRelativeLocation` _interactingobj (`KismetMathLibrary.VLerp` (`KismetMathLibrary.MakeVector` 0.0 0.0 _relativelocation_z) (`KismetMathLibrary.MakeVector` 0.0 (`self.OpenDistance`) _relativelocation_z) _alpha) false false))
    (:`Finished`
      (set `/Game/ThirdPersonBP/Blueprints/ThirdPersonCharacter.bIsTimelinePlaying?` false _playerref))))

(event `CloseDrawer`
  (`TimelineComponent.SetPlaybackPosition` (`self.Open`) 1.0 false true)
  (goto _label_2 :!via `Reverse`))

(fn `UserConstructionScript`)