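; BP_SimpleDoor is an interactable door that opens and closes with skeletal mesh animations and can require an item while locked.
; Interact checks the lock and required item, then a FlipFlop alternates between DoorOpen and DoorClose.
; Each animation clears Usable for a fixed delay to block repeated use.
; The first close also calls CallStreamLevel1 once through a DoOnce.
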(event `DoorOpen`
  ;[1 1 1] DoorOpen
  (set `self.Usable?` false)
  (`SkeletalMeshComponent.PlayAnimation` (`self.SkeletalMesh`) "/Game/HQ_ResidentialHouse/Meshes/DoorNarrow/Door_narrow_Anim.Door_narrow_Anim" false)
  (`KismetSystemLibrary.Delay` 3.0)
  (set `self.Usable?` true))

(event `DoorClose`
  ;[1 1 1] DoorClose
  (set `self.Usable?` false)
  (`SkeletalMeshComponent.PlayAnimation` (`self.SkeletalMesh`) "/Game/HQ_ResidentialHouse/Meshes/DoorNarrow/Door_narrowClose_Anim.Door_narrowClose_Anim" false)
  (`|ExecutionSequence`
    (:`then_0`
      (`/Engine/EditorBlueprintResources/StandardMacros.DoOnce` false
        (:`Completed`
          (`self.StreamLevel1`))))
    (:`then_1`
      (`KismetSystemLibrary.Delay` 3.0)
      (set `self.Usable?` true))))

(event `/Game/Sunny_TestingArea/Interactables/BPI_Interact.Interact`
  (params (InteractingComponent :type "PrimitiveComponent Object Reference (by ref)"))
  ;[1 1 1] DoorInteract
  (if (`self.Locked?`)
    (if (`/Game/Sunny_TestingArea/Interactables/BPFL_Interact.CheckHasRequiredItem?` (`self.Tags`))
      (if (`self.Usable?`) :!label _label
        (`/Engine/EditorBlueprintResources/StandardMacros.FlipFlop`
          (:`A`
            (`self.DoorOpen`))
          (:`B`
            (`self.DoorClose`)))))
    (else
      (goto _label))))

(fn `UserConstructionScript`)