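; Interactable fusebox with a lockable door that opens with a key item and accepts a fuse from the player's inventory.
; Interact unlocks, toggles the timeline-driven door or, when fully open, inserts the fuse.
; Key and fuse animations spawn temporary mesh actors lerped into sockets; the fuse's completion reveals a switch and removes the item.
; Physics-door auto-close logic remains, but its distance check is disconnected.
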(event `FuseAnim`
  (bind (_returnvalue_location _returnvalue_rotation _returnvalue_scale) (`KismetMathLibrary.BreakTransform` (`SceneComponent.GetSocketTransform` (`self.Interior`) (`self.FuseSocketName`) "RTS_World")))
  (bind _inventory (`/Game/ThirdPersonBP/Blueprints/ThirdPersonCharacter.Inventory` (`self.PlayerRef`)))
  ;[1 1 1] Animation for fuse into fuse box
  (bind _returnvalue (`|SpawnActorFromClass` "/Script/Engine.StaticMeshActor" (`KismetMathLibrary.MakeTransform` (+ _returnvalue_location (`self.FuseSpawnDistance`)) _returnvalue_rotation _returnvalue_scale) "Undefined" "OverrideRootScale" null null))
  (bind _output_get (set `self.StaticMeshRef` _returnvalue))
  (`StaticMeshActor.SetMobility` _output_get "Movable")
  (bind _returnvalue_2 (`StaticMeshComponent.SetStaticMesh` (`StaticMeshActor.StaticMeshComponent` _output_get) (`self.FuseMesh`)))
  (if _returnvalue_2
    (`self.SetActorEnableCollision` _output_get false)
    (bind (_direction _transformalpha _rotationalpha) (`Timeline|Timeline_0`)
      (:`Update`
        (bind _rotation (.rotation (`KismetMathLibrary.TLerp` (`self.GetTransform` (`self.StaticMeshRef`)) (`SceneComponent.GetSocketTransform` (`self.Interior`) (`self.FuseSocketName`) "RTS_World") _transformalpha)))
        (`self.K2_SetActorTransform` (`self.StaticMeshRef`) (`KismetMathLibrary.MakeTransform` (.location (`KismetMathLibrary.TLerp` (`self.GetTransform` (`self.StaticMeshRef`)) (`SceneComponent.GetSocketTransform` (`self.Interior`) (`self.FuseSocketName`) "RTS_World") _transformalpha)) (`KismetMathLibrary.RLerp` _rotation (`KismetMathLibrary.ComposeRotators` _rotation (struct :`Pitch` -35.0)) _rotationalpha) (.scale (`KismetMathLibrary.TLerp` (`self.GetTransform` (`self.StaticMeshRef`)) (`SceneComponent.GetSocketTransform` (`self.Interior`) (`self.FuseSocketName`) "RTS_World") _transformalpha))) false false))
      (:`Finished`
        (`SceneComponent.SetVisibility` (`self.Switch1`) true false)
        (`self.K2_DestroyActor` (`self.StaticMeshRef`))
        (for (_array_element _array_index) _inventory
          (if (== (`.ItemTag_15_66EBFC3A46588EAB875FE09C56D5FF94` (break `/Game/UMG/S_InventoryItems` _array_element)) (`self.FuseTag`))
            (`KismetArrayLibrary.Array_Remove` _inventory _array_index)))))))

(event `self.ReceiveBeginPlay`
  ;[1 1 1] Event Begin Play
  (bind _asthird_person_character (cast `/Game/ThirdPersonBP/Blueprints/ThirdPersonCharacter` (`GameplayStatics.GetPlayerCharacter` 0)))
  (set `self.PlayerRef` _asthird_person_character)
  (set `self.DefaultRotation` (`SceneComponent.RelativeRotation` (`self.Door`))))

(event `UnlockDoor`
  (bind (_returnvalue_location _returnvalue_rotation _returnvalue_scale) (`KismetMathLibrary.BreakTransform` (`SceneComponent.GetSocketTransform` (`self.Door`) (`self.KeySocketName`) "RTS_World")))
  ;[1 1 1] Animation for key unlocking door
  (bind _returnvalue (`|SpawnActorFromClass` "/Script/Engine.StaticMeshActor" (`KismetMathLibrary.MakeTransform` (+ _returnvalue_location (`self.KeySpawnDistance`)) _returnvalue_rotation _returnvalue_scale) "Undefined" "OverrideRootScale" null null))
  (bind _output_get (set `self.StaticMeshRef` _returnvalue))
  (`StaticMeshActor.SetMobility` _output_get "Movable")
  (bind _returnvalue_2 (`StaticMeshComponent.SetStaticMesh` (`StaticMeshActor.StaticMeshComponent` _output_get) (`self.KeyMesh`)))
  (if _returnvalue_2
    (`self.SetActorEnableCollision` _output_get false)
    (bind (_direction _transformalpha _rotationalpha) (`Timeline|Unlock`)
      (:`Update`
        (bind _rotation (.rotation (`KismetMathLibrary.TLerp` (`self.GetTransform` (`self.StaticMeshRef`)) (`SceneComponent.GetSocketTransform` (`self.Door`) (`self.KeySocketName`) "RTS_World") _transformalpha)))
        (`self.K2_SetActorTransform` (`self.StaticMeshRef`) (`KismetMathLibrary.MakeTransform` (.location (`KismetMathLibrary.TLerp` (`self.GetTransform` (`self.StaticMeshRef`)) (`SceneComponent.GetSocketTransform` (`self.Door`) (`self.KeySocketName`) "RTS_World") _transformalpha)) (`KismetMathLibrary.RLerp` _rotation (`KismetMathLibrary.ComposeRotators` _rotation (struct :`Roll` -90.0)) _rotationalpha true) (.scale (`KismetMathLibrary.TLerp` (`self.GetTransform` (`self.StaticMeshRef`)) (`SceneComponent.GetSocketTransform` (`self.Door`) (`self.KeySocketName`) "RTS_World") _transformalpha))) false false))
      (:`Finished`
        (set `self.Locked?` false)
        (`self.K2_DestroyActor` (`self.StaticMeshRef`))
        (`/Game/Sunny_TestingArea/Interactables/BPI_Interact.Interact` (`self.Door`))))))

(event `/Game/Sunny_TestingArea/Interactables/BPI_Interact.Interact`
  (params (InteractingComponent :type "PrimitiveComponent Object Reference (by ref)"))
  (bind _relativerotation (`SceneComponent.RelativeRotation` (`self.Door`)))
  ;[1 1 1] Enables the physics for the door
  (if (`self.Locked?`)
    (if (`/Game/Sunny_TestingArea/Interactables/BPFL_Interact.CheckHasRequiredItem?` (`self.Tags`))
      (`self.UnlockDoor`))
    (elif (== _relativerotation (struct :`Yaw` 90.0) :`ErrorTolerance` 0.1)
      (if (`/Game/Sunny_TestingArea/Interactables/BPFL_Interact.CheckHasRequiredItem?` (`self.Tags`) (`self.FuseTag`))
        (`self.FuseAnim`)
        (else
          (if (!= _relativerotation (`self.DefaultRotation`) :`ErrorTolerance` 0.1) :!label _label
            (`self.CloseDoor`)
            (else
              (`self.OpenDoor`)))))
      (else
        (goto _label)))))

(event `/Game/Sunny_TestingArea/Interactables/BPI_Interact.DisablePhysics`
  ;[1 1 1] Distance check for door (if auto close is turned on)
)

(event `OpenDoor`
  (bind _playerref (`self.PlayerRef`))
  ;[1 1 1] open and close door without physics
  (`PrimitiveComponent.SetSimulatePhysics` (`self.Door`) false)
  (`TimelineComponent.SetPlaybackPosition` (`self.Open`) 0.0 false true)
  (set `self.OpenDir` 90.0)
  (bind (_direction _alpha) (`Timeline|Open` :!label _label_2)
    (:`Update`
      (set `/Game/ThirdPersonBP/Blueprints/ThirdPersonCharacter.bIsTimelinePlaying?` true _playerref)
      (`SceneComponent.K2_SetRelativeRotation` (`self.Door`) (`KismetMathLibrary.RLerp` (`self.DefaultRotation`) (`KismetMathLibrary.MakeRotator` 0.0 0.0 (`self.OpenDir`)) _alpha) false false)
      (set `self.DoorClosed?` false))
    (:`Finished`
      (set `/Game/ThirdPersonBP/Blueprints/ThirdPersonCharacter.bIsTimelinePlaying?` false _playerref)
      (set `self.DoorClosed?` true))))

(event `CloseDoor`
  ;[1 1 1] open and close door without physics
  (`PrimitiveComponent.SetSimulatePhysics` (`self.Door`) (`self.PhysicsInteraction?`))
  (`TimelineComponent.SetPlaybackPosition` (`self.Open`) 1.0 false true)
  (goto _label_2 :!via `Reverse`))

(event `AutoCloseDoor`
  ;[1 1 1] Close Door (used for both with and without physics)
  (if (`self.ShouldAutoClose?`)
    (bind (_direction _alpha) (`Timeline|AutoClose`)
      (:`Update`
        (`SceneComponent.K2_SetWorldRotation` (`self.Door`) (`KismetMathLibrary.RLerp` (`self.DoorCurrentRot`) (`self.DefaultRotation`) _alpha) false false))
      (:`Finished`
        (`TimelineComponent.SetPlaybackPosition` (`self.AutoClose`) 0.0 false false :!label _label_3)
        (set `self.DoorClosed?` true)
        (`PrimitiveComponent.SetSimulatePhysics` (`self.Door`) false)))
    (else
      (`TimelineComponent.Stop` (`self.DistanceCheck`))
      (goto _label_3))))

(fn `IsDoorOpen?`
  (returns (Return :type Boolean))
  (bind (_defaultrotation_roll _defaultrotation_pitch _defaultrotation_yaw) (`KismetMathLibrary.BreakRotator` (`self.DefaultRotation`)))
  (bind (_returnvalue_roll _returnvalue_pitch _returnvalue_yaw) (`KismetMathLibrary.BreakRotator` (`SceneComponent.K2_GetComponentRotation` (`self.Door`))))
  (return (select `bool` (> (`self.GetHorizontalDotProductTo` self (`GameplayStatics.GetPlayerCharacter` 0)) 0.0) :`false` (< _returnvalue_yaw _defaultrotation_yaw) :`true` (> _returnvalue_yaw _defaultrotation_yaw))))

(fn `UserConstructionScript`
  (`PrimitiveComponent.SetSimulatePhysics` (`self.Door`) (`self.PhysicsInteraction?`)))