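; Interactable sliding object, such as a drawer, that opens or closes when interacted with, requiring an item check if locked.
; Interact toggles by whether the mesh sits at its relative origin, playing or reversing a timeline lerp along the chosen axis, optionally flipped.
; The timeline's play rate comes from Speed, and it flags the player while running.
; The construction script applies the mesh and positions an arrow previewing the opening direction and distance.
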(event `self.ReceiveBeginPlay`
  (bind _asthird_person_character (cast `/Game/ThirdPersonBP/Blueprints/ThirdPersonCharacter` (`GameplayStatics.GetPlayerCharacter` 0)))
  (set `self.PlayerRef` _asthird_person_character)
  (set `self.MeshesToAffect` (`|MakeArray` (`self.StaticMesh1`)))
  (`TimelineComponent.SetPlayRate` (`self.Open`) (`self.Speed`)))

(event `/Game/Sunny_TestingArea/Interactables/BPI_Interact.Interact`
  (params (InteractingComponent :type "PrimitiveComponent Object Reference (by ref)"))
  ;[1 1 1] Check if the drawer is opened or close (if the drawer's location is equal to the location+distance then the drawer is open so close it)
  (for _array_element (`self.MeshesToAffect`)
    (if (== _array_element InteractingComponent)
      (set `self.InteractingObj` _array_element)))
  (if (`self.Locked?`)
    (if (`/Game/Sunny_TestingArea/Interactables/BPFL_Interact.CheckHasRequiredItem?` (`self.Tags`))
      (if (!= (`SceneComponent.RelativeLocation` (`self.InteractingObj`)) (0.0 0.0 0.0) :`ErrorTolerance` 1.0) :!label _label
        (`self.CloseDrawer`)
        (else
          (`self.OpenDrawer`))))
    (else
      (goto _label))))

(event `OpenDrawer`
  (bind _opendistance (`self.OpenDistance`))
  (bind _playerref (`self.PlayerRef`))
  (bind _returnvalue (select `bool` (`self.FlipOpeningDirection?`) :`false` _opendistance :`true` (* _opendistance -1.0)))
  ;[1 1 1] Just a basic timeline that opens and closes the drawer using a lerp
  (`TimelineComponent.SetPlaybackPosition` (`self.Open`) 0.0 false true)
  (bind (_direction _alpha) (`Timeline|Open` :!label _label_2)
    (:`Update`
      (set `/Game/ThirdPersonBP/Blueprints/ThirdPersonCharacter.bIsTimelinePlaying?` true _playerref)
      (`SceneComponent.K2_SetRelativeLocation` (`self.InteractingObj`) (`KismetMathLibrary.VLerp` (`KismetMathLibrary.MakeVector` 0.0) (select `/Game/Sunny_TestingArea/E_Direction` (`self.Direction`) :`NewEnumerator0` (`KismetMathLibrary.MakeVector` 0.0 _returnvalue) :`NewEnumerator1` (`KismetMathLibrary.MakeVector` _returnvalue) :`NewEnumerator2` (`KismetMathLibrary.MakeVector` 0.0 0.0 _returnvalue)) _alpha) false false))
    (:`Finished`
      (set `/Game/ThirdPersonBP/Blueprints/ThirdPersonCharacter.bIsTimelinePlaying?` false _playerref))))

(event `CloseDrawer`
  ;[1 1 1] Just a basic timeline that opens and closes the drawer using a lerp
  (`TimelineComponent.SetPlaybackPosition` (`self.Open`) 1.0 false true)
  (goto _label_2 :!via `Reverse`))

(fn `UserConstructionScript`
  (bind _opendistance (`self.OpenDistance`))
  (bind _direction (`self.Direction`))
  (bind (_relativelocation_x _relativelocation_y _relativelocation_z) (`KismetMathLibrary.BreakVector` (`SceneComponent.RelativeLocation` (`self.Arrow`))))
  (bind _returnvalue (select `bool` (`self.FlipOpeningDirection?`) :`false` _opendistance :`true` (* _opendistance -1.0)))
  (bind _returnvalue_2 (`KismetMathLibrary.MakeVector` _relativelocation_x _relativelocation_y _returnvalue))
  (bind _returnvalue_3 (`KismetMathLibrary.MakeVector` _relativelocation_x _returnvalue _relativelocation_z))
  (bind _returnvalue_4 (`KismetMathLibrary.MakeVector` _returnvalue _relativelocation_y _relativelocation_z))
  (`StaticMeshComponent.SetStaticMesh` (`self.StaticMesh1`) (`self.QuickNewMesh`))
  (`SceneComponent.K2_SetRelativeLocationAndRotation` (`self.Arrow`) (select `/Game/Sunny_TestingArea/E_Direction` _direction :`NewEnumerator0` _returnvalue_3 :`NewEnumerator1` _returnvalue_4 :`NewEnumerator2` _returnvalue_2) (select `/Game/Sunny_TestingArea/E_Direction` _direction :`NewEnumerator0` (`KismetMathLibrary.MakeRotationFromAxes` _returnvalue_3 _returnvalue_4 _returnvalue_2) :`NewEnumerator1` (`KismetMathLibrary.MakeRotFromX` _returnvalue_4) :`NewEnumerator2` (`KismetMathLibrary.MakeRotationFromAxes` _returnvalue_2 _returnvalue_4 _returnvalue_3)) false false))