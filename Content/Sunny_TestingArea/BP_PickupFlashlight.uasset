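; BP_PickupFlashlight is a pickup actor that gives the player a flashlight.
; BeginPlay creates a dynamic material instance on its static mesh and sets a grey emissive light color.
; Interact casts the player to ThirdPersonCharacter, sets its PickedupFlashlight flag, shows its SpotLight and destroys the pickup.
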(event `self.ReceiveBeginPlay`
  (bind _returnvalue (`PrimitiveComponent.CreateDynamicMaterialInstance` (`self.StaticMesh`) 0 "/Game/phong3.phong3" "None"))
  (`MaterialInstanceDynamic.SetVectorParameterValue` _returnvalue "EmissiveLightColor" (struct :`R` 0.463542 :`G` 0.463542 :`B` 0.463542 :`A` 0.75)))

(event `/Game/Sunny_TestingArea/Interactables/BPI_Interact.Interact`
  (bind _asthird_person_character (cast `/Game/ThirdPersonBP/Blueprints/ThirdPersonCharacter` (`GameplayStatics.GetPlayerCharacter` 0)))
  (set `/Game/ThirdPersonBP/Blueprints/ThirdPersonCharacter.bPickedupFlashlight?` true _asthird_person_character)
  (`SceneComponent.SetVisibility` (`/Game/ThirdPersonBP/Blueprints/ThirdPersonCharacter.SpotLight` _asthird_person_character) true false)
  (`self.K2_DestroyActor`))

(fn `UserConstructionScript`)