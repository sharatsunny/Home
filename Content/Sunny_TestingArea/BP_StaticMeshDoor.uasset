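; Interactable static mesh door Blueprint that swings open or closed on Interact, with an optional lock gated by a required-item tag check.
; A dot product with the player picks a positive or negative 90-degree swing when opening.
; The OpenDoor timeline lerps the mesh's relative yaw, and reverses to close when the mesh is already fully open.
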(event `/Game/Sunny_TestingArea/Interactables/BPI_Interact.Interact`
  (params (InteractingComponent :type "PrimitiveComponent Object Reference (by ref)"))
  (bind _relativerotation (`SceneComponent.RelativeRotation` (`self.StaticMesh`)))
  (if (`self.Locked?`)
    (if (`/Game/Sunny_TestingArea/Interactables/BPFL_Interact.CheckHasRequiredItem?` (`self.Tags`))
      (if (or (== _relativerotation (struct :`Yaw` 90.0) :`ErrorTolerance` 0.1) (== _relativerotation (struct :`Yaw` -90.0) :`ErrorTolerance` 0.1)) :!label _label
        (bind (_direction _alpha) (`Timeline|OpenDoor` :!via `Reverse` :!label _label_2)
          (:`Update`
            (`SceneComponent.K2_SetRelativeRotation` (`self.StaticMesh`) (`KismetMathLibrary.MakeRotator` 0.0 0.0 (`KismetMathLibrary.Lerp` 0.0 (`self.OpenDir`) _alpha)) false false)))
        (else
          (set `self.OpenDir` (`KismetMathLibrary.SelectFloat` -90.0 90.0 (and (> (`self.GetHorizontalDotProductTo` self (`GameplayStatics.GetPlayerCharacter` 0)) 0.0) (!= (`TimelineComponent.GetPlaybackPosition` (`self.OpenDoor`)) 1.0))))
          (goto _label_2))))
    (else
      (goto _label))))

(fn `UserConstructionScript`)