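; BP_PhysicsDoor is an interactable door that the player swings with an axis input, optionally locked behind a required item.
; Interact enables mesh physics, and PhysicsInteraction adds yaw, using a dot product to pick direction by player side and clamp at the closed rotation.
; DisablePhysics snaps a nearly closed door shut, otherwise a timeline monitors player distance and triggers CloseDoor, which lerps it back to its initial rotation.
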(event `self.ReceiveBeginPlay`
  (bind _asthird_person_character (cast `/Game/ThirdPersonBP/Blueprints/ThirdPersonCharacter` (`GameplayStatics.GetPlayerCharacter` 0)))
  (set `self.PlayerRef` _asthird_person_character)
  (set `self.DefaultRotation` (`SceneComponent.K2_GetComponentRotation` (`self.StaticMesh1`))))

(event `/Game/Sunny_TestingArea/Interactables/BPI_Interact.Interact`
  (params (InteractingComponent :type "PrimitiveComponent Object Reference (by ref)"))
  (bind (_defaultrotation_roll _defaultrotation_pitch _defaultrotation_yaw) (`KismetMathLibrary.BreakRotator` (`self.DefaultRotation`)))
  (bind (_returnvalue_roll _returnvalue_pitch _returnvalue_yaw) (`KismetMathLibrary.BreakRotator` (`SceneComponent.K2_GetComponentRotation` (`self.StaticMesh1`))))
  ;[1 1 1] Enables the physics for the door
  (if (`self.Locked?`)
    (if (`/Game/Sunny_TestingArea/Interactables/BPFL_Interact.CheckHasRequiredItem?` (`self.Tags`))
      (set `/Game/ThirdPersonBP/Blueprints/ThirdPersonCharacter.bIsPhysicsInteraction?` true (`self.PlayerRef`) :!label _label)
      (`PrimitiveComponent.SetSimulatePhysics` (`self.StaticMesh1`) true)
      (if (select `bool` (> (`self.GetHorizontalDotProductTo` self (`GameplayStatics.GetPlayerCharacter` 0)) 0.0) :`false` (< _returnvalue_yaw _defaultrotation_yaw) :`true` (> _returnvalue_yaw _defaultrotation_yaw))
        (`self.CloseDoor`)))
    (else
      (goto _label))))

(event `/Game/Sunny_TestingArea/Interactables/BPI_Interact.PhysicsInteraction`
  (params (XValue :type "Float (single-precision)") (YValue :type "Float (single-precision)"))
  (bind (_defaultrotation_roll _defaultrotation_pitch _defaultrotation_yaw) (`KismetMathLibrary.BreakRotator` (`self.DefaultRotation`)))
  (bind (_returnvalue_roll _returnvalue_pitch _returnvalue_yaw) (`KismetMathLibrary.BreakRotator` (`SceneComponent.K2_GetComponentRotation` (`self.StaticMesh1`))))
  (bind _returnvalue (* YValue (`self.SpeedMultiplier`)))
  (bind _returnvalue_2 (> (`self.GetHorizontalDotProductTo` self (`GameplayStatics.GetPlayerCharacter` 0)) 0.0))
  ;[1 1 1] rotates the door based on the mouse axis value
  (if (`self.Locked?`)
    (if (`/Game/Sunny_TestingArea/Interactables/BPFL_Interact.CheckHasRequiredItem?` (`self.Tags`))
      (if (select `bool` _returnvalue_2 :`false` (< _returnvalue_yaw _defaultrotation_yaw) :`true` (> _returnvalue_yaw _defaultrotation_yaw)) :!label _label_2
        (`SceneComponent.K2_SetWorldRotation` (`self.StaticMesh1`) (`self.DefaultRotation`) false false)
        (set `self.DoorClosed?` true)
        (else
          (`SceneComponent.K2_AddWorldRotation` (`self.StaticMesh1`) (`KismetMathLibrary.MakeRotator` 0.0 0.0 (`KismetMathLibrary.SelectFloat` _returnvalue (* _returnvalue -1.0) _returnvalue_2)) false false)
          (set `self.DoorClosed?` false))))
    (else
      (goto _label_2))))

(event `/Game/Sunny_TestingArea/Interactables/BPI_Interact.DisablePhysics`
  (bind (_defaultrotation_roll _defaultrotation_pitch _defaultrotation_yaw) (`KismetMathLibrary.BreakRotator` (`self.DefaultRotation`)))
  (bind (_returnvalue_roll _returnvalue_pitch _returnvalue_yaw) (`KismetMathLibrary.BreakRotator` (`SceneComponent.K2_GetComponentRotation` (`self.StaticMesh1`))))
  (bind _returnvalue (`self.GetDistanceTo` (`self.PlayerRef`) self))
  ;[1 1 1] Do a bunch of checks and close door if it's left opened or if the door is close to it's original rotation
  (set `self.DoorCurrentRot` (`SceneComponent.K2_GetComponentRotation` (`self.StaticMesh1`)))
  (if (and (not (`/Game/ThirdPersonBP/Blueprints/ThirdPersonCharacter.bIsPhysicsInteraction?` (`self.PlayerRef`))) (`KismetMathLibrary.NearlyEqual_FloatFloat` _returnvalue_yaw _defaultrotation_yaw 10.0)) :!label _label_3
    (`SceneComponent.K2_SetWorldRotation` (`self.StaticMesh1`) (`self.DefaultRotation`) false false)
    (`PrimitiveComponent.SetSimulatePhysics` (`self.StaticMesh1`) false)
    (set `self.DoorClosed?` true)
    (`Timeline|Timeline_0` :!via `Stop` :!label _label_4
      (:`Update`
        (if (> _returnvalue 1000.0)
          (goto _label_4 :!via `Stop`)
          (elif (> _returnvalue 300.0)
            (if (not (`self.DoorClosed?`))
              (`self.CloseDoor`))
            (else
              (set `self.DoorClosed?` false)
              (goto _label_3))))))
    (else
      (goto _label_4))))

(event `CloseDoor`
  ;[1 1 1] Close Door
  (`PrimitiveComponent.SetSimulatePhysics` (`self.StaticMesh1`) false)
  (bind (_direction _alpha) (`Timeline|AutoCloseDoor`)
    (:`Update`
      (`SceneComponent.K2_SetWorldRotation` (`self.StaticMesh1`) (`KismetMathLibrary.RLerp` (`self.DoorCurrentRot`) (`self.DefaultRotation`) _alpha) false false))
    (:`Finished`
      (`TimelineComponent.SetPlaybackPosition` (`self.AutoCloseDoor`) 0.0 false false)
      (set `self.DoorClosed?` true))))

(fn `UserConstructionScript`)