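; Interactive door Blueprint that can be lockable and opens either through a timeline swing or physics-driven player input.
; When the required-item check passes, Interact spawns a key mesh at a socket, animates its turn, then unlocks.
; A dot product against the player picks swing direction, and physics pushing snaps shut on crossing the default yaw.
; Timelines drive opening, closing and distance-checked optional auto-close, while flags on ThirdPersonCharacter track interaction state.
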(event `self.ReceiveBeginPlay`
  (bind _staticmesh1 (`self.StaticMesh1`))
  ;[1 1 1] Event Begin Play
  (bind _asthird_person_character (cast `/Game/ThirdPersonBP/Blueprints/ThirdPersonCharacter` (`GameplayStatics.GetPlayerCharacter` 0)))
  (set `self.PlayerRef` _asthird_person_character)
  (set `self.DefaultWorldRotation` (`SceneComponent.K2_GetComponentRotation` _staticmesh1))
  (set `self.DefaultRelativeRotation` (`SceneComponent.RelativeRotation` _staticmesh1)))

(event `UnlockDoor`
  (bind (_returnvalue_location _returnvalue_rotation _returnvalue_scale) (`KismetMathLibrary.BreakTransform` (`SceneComponent.GetSocketTransform` (`self.StaticMesh1`) (`self.KeySocketName`) "RTS_World")))
  ;[1 1 1] Animation for key unlocking door
  (bind _returnvalue (`|SpawnActorFromClass` "/Script/Engine.StaticMeshActor" (`KismetMathLibrary.MakeTransform` (+ _returnvalue_location (`self.KeySpawnDistance`)) _returnvalue_rotation _returnvalue_scale) "Undefined" "OverrideRootScale" null null))
  (bind _output_get (set `self.KeyMeshRef` _returnvalue))
  (`StaticMeshActor.SetMobility` _output_get "Movable")
  (bind _returnvalue_2 (`StaticMeshComponent.SetStaticMesh` (`StaticMeshActor.StaticMeshComponent` _output_get) (`self.KeyMesh`)))
  (if _returnvalue_2
    (`self.SetActorEnableCollision` _output_get false)
    (bind (_direction _transformalpha _rotationalpha) (`Timeline|Unlock`)
      (:`Update`
        (bind _rotation (.rotation (`KismetMathLibrary.TLerp` (`self.GetTransform` (`self.KeyMeshRef`)) (`SceneComponent.GetSocketTransform` (`self.StaticMesh1`) (`self.KeySocketName`) "RTS_World") _transformalpha)))
        (`self.K2_SetActorTransform` (`self.KeyMeshRef`) (`KismetMathLibrary.MakeTransform` (.location (`KismetMathLibrary.TLerp` (`self.GetTransform` (`self.KeyMeshRef`)) (`SceneComponent.GetSocketTransform` (`self.StaticMesh1`) (`self.KeySocketName`) "RTS_World") _transformalpha)) (`KismetMathLibrary.RLerp` _rotation (`KismetMathLibrary.ComposeRotators` _rotation (struct :`Roll` 90.0)) _rotationalpha) (.scale (`KismetMathLibrary.TLerp` (`self.GetTransform` (`self.KeyMeshRef`)) (`SceneComponent.GetSocketTransform` (`self.StaticMesh1`) (`self.KeySocketName`) "RTS_World") _transformalpha))) false false))
      (:`Finished`
        (set `self.Locked?` false)
        (`self.K2_DestroyActor` (`self.KeyMeshRef`))
        (`/Game/Sunny_TestingArea/Interactables/BPI_Interact.Interact` (`self.StaticMesh1`))))))

(event `/Game/Sunny_TestingArea/Interactables/BPI_Interact.Interact`
  (params (InteractingComponent :type "PrimitiveComponent Object Reference (by ref)"))
  (bind _return (`self.IsDoorOpen?`))
  ;[1 1 1] Enables the physics for the door
  (if (`self.Locked?`)
    (if (`/Game/Sunny_TestingArea/Interactables/BPFL_Interact.CheckHasRequiredItem?` (`self.Tags`))
      (`self.UnlockDoor`))
    (elif (`self.PhysicsInteraction?`)
      (set `/Game/ThirdPersonBP/Blueprints/ThirdPersonCharacter.bIsPhysicsInteraction?` true (`self.PlayerRef`))
      (if _return
        (`self.AutoCloseDoor`))
      (elif _return
        (`self.CloseDoor` :!label _label)
        (elif (!= (`SceneComponent.RelativeRotation` (`self.StaticMesh1`)) (`self.DefaultRelativeRotation`) :`ErrorTolerance` 0.1)
          (goto _label)
          (else
            (`self.OpenDoor`)))))))

(event `OpenDoor`
  (bind _playerref (`self.PlayerRef`))
  ;[1 1 1] open and close door without physics
  (`PrimitiveComponent.SetSimulatePhysics` (`self.StaticMesh1`) false)
  (`TimelineComponent.SetPlaybackPosition` (`self.Open`) 0.0 false true)
  (set `self.OpenDir` (select `bool` (> (`self.GetHorizontalDotProductTo` self (`GameplayStatics.GetPlayerCharacter` 0)) 0.0) :`false` 90.0 :`true` -90.0 :!type "Float (single-precision)"))
  (bind (_direction _alpha) (`Timeline|Open` :!label _label_2)
    (:`Update`
      (set `/Game/ThirdPersonBP/Blueprints/ThirdPersonCharacter.bIsTimelinePlaying?` true _playerref)
      (`SceneComponent.K2_SetRelativeRotation` (`self.StaticMesh1`) (`KismetMathLibrary.RLerp` (`self.DefaultRelativeRotation`) (`KismetMathLibrary.MakeRotator` 0.0 0.0 (`self.OpenDir`)) _alpha) false false)
      (set `self.DoorClosed?` false))
    (:`Finished`
      (set `/Game/ThirdPersonBP/Blueprints/ThirdPersonCharacter.bIsTimelinePlaying?` false _playerref)
      (set `self.DoorClosed?` true))))

(event `/Game/Sunny_TestingArea/Interactables/BPI_Interact.PhysicsInteraction`
  (params (XValue :type "Float (single-precision)") (YValue :type "Float (single-precision)"))
  (bind _staticmesh1 (`self.StaticMesh1`))
  (bind (_defaultworldrotation_roll _defaultworldrotation_pitch _defaultworldrotation_yaw) (`KismetMathLibrary.BreakRotator` (`self.DefaultWorldRotation`)))
  (bind (_doorcurrentrot_roll _doorcurrentrot_pitch _doorcurrentrot_yaw) (`KismetMathLibrary.BreakRotator` (`self.DoorCurrentRot`)))
  (bind (_returnvalue_roll _returnvalue_pitch _returnvalue_yaw) (`KismetMathLibrary.BreakRotator` (`SceneComponent.K2_GetComponentRotation` (`self.StaticMesh1`))))
  (bind _returnvalue (* YValue (`self.SpeedMultiplier`)))
  (bind _returnvalue_2 (> (`self.GetHorizontalDotProductTo` self (`GameplayStatics.GetPlayerCharacter` 0)) 0.0))
  ;[1 1 1] Open door with physics (this also makes sure the player can only open the door away from the player not towards the player)
  (set `self.DoorCurrentRot` (`SceneComponent.K2_GetComponentRotation` (`self.StaticMesh1`)))
  (if (`self.Locked?`)
    (if (`/Game/Sunny_TestingArea/Interactables/BPFL_Interact.CheckHasRequiredItem?` (`self.Tags`))
      (if (`KismetMathLibrary.NearlyEqual_FloatFloat` (`self.GetHorizontalDotProductTo` self (`GameplayStatics.GetPlayerCharacter` 0)) 0.0 0.1) :!label _label_3
        (`self.AutoCloseDoor`)
        (else
          (`PrimitiveComponent.SetSimulatePhysics` _staticmesh1 true)
          (`SceneComponent.K2_AddWorldRotation` _staticmesh1 (`KismetMathLibrary.MakeRotator` 0.0 0.0 (`KismetMathLibrary.SelectFloat` _returnvalue (* _returnvalue -1.0) _returnvalue_2)) false true)
          (set `self.DoorClosed?` false)
          (if (and (>= _returnvalue_yaw _defaultworldrotation_yaw) (<= _doorcurrentrot_yaw _defaultworldrotation_yaw) _returnvalue_2)
            (`SceneComponent.K2_SetWorldRotation` (`self.StaticMesh1`) (`self.DefaultWorldRotation`) false true :!label _label_4)
            (set `self.DoorClosed?` true)
            (elif (and (<= _returnvalue_yaw _defaultworldrotation_yaw) (>= _doorcurrentrot_yaw _defaultworldrotation_yaw) (not _returnvalue_2))
              (goto _label_4))))))
    (else
      (goto _label_3))))

(event `CloseDoor`
  ;[1 1 1] open and close door without physics
  (`PrimitiveComponent.SetSimulatePhysics` (`self.StaticMesh1`) (`self.PhysicsInteraction?`))
  (`TimelineComponent.SetPlaybackPosition` (`self.Open`) 1.0 false true)
  (goto _label_2 :!via `Reverse`))

(event `/Game/Sunny_TestingArea/Interactables/BPI_Interact.DisablePhysics`
  (bind (_defaultworldrotation_roll _defaultworldrotation_pitch _defaultworldrotation_yaw) (`KismetMathLibrary.BreakRotator` (`self.DefaultWorldRotation`)))
  (bind (_returnvalue_roll _returnvalue_pitch _returnvalue_yaw) (`KismetMathLibrary.BreakRotator` (`SceneComponent.K2_GetComponentRotation` (`self.StaticMesh1`))))
  (bind _returnvalue (`self.GetDistanceTo` (`self.PlayerRef`) self))
  ;[1 1 1] Distance check for door (if auto close is turned on)
  (set `self.DoorCurrentRot` (`SceneComponent.K2_GetComponentRotation` (`self.StaticMesh1`)))
  (if (and (not (`/Game/ThirdPersonBP/Blueprints/ThirdPersonCharacter.bIsPhysicsInteraction?` (`self.PlayerRef`))) (`KismetMathLibrary.NearlyEqual_FloatFloat` _returnvalue_yaw _defaultworldrotation_yaw 10.0)) :!label _label_5
    (`SceneComponent.K2_SetWorldRotation` (`self.StaticMesh1`) (`self.DefaultWorldRotation`) false true)
    (`PrimitiveComponent.SetSimulatePhysics` (`self.StaticMesh1`) false)
    (set `self.DoorClosed?` true)
    (`Timeline|DistanceCheck` :!via `Stop` :!label _label_6
      (:`Update`
        (if (> _returnvalue 1000.0)
          (goto _label_6 :!via `Stop`)
          (elif (> _returnvalue 300.0)
            (if (not (`self.DoorClosed?`))
              (`self.AutoCloseDoor`))
            (else
              (set `self.DoorClosed?` false)
              (goto _label_5))))))
    (else
      (goto _label_6))))

(event `AutoCloseDoor`
  ;[1 1 1] Close Door (used for both with and without physics)
  (if (`self.ShouldAutoClose?`)
    (bind (_direction _alpha) (`Timeline|AutoClose`)
      (:`Update`
        (`SceneComponent.K2_SetWorldRotation` (`self.StaticMesh1`) (`KismetMathLibrary.RLerp` (`self.DoorCurrentRot`) (`self.DefaultWorldRotation`) _alpha) false false))
      (:`Finished`
        (`TimelineComponent.SetPlaybackPosition` (`self.AutoClose`) 0.0 false false :!label _label_7)
        (set `self.DoorClosed?` true)
        (`PrimitiveComponent.SetSimulatePhysics` (`self.StaticMesh1`) false)))
    (else
      (`TimelineComponent.Stop` (`self.DistanceCheck`))
      (goto _label_7))))

(fn `IsDoorOpen?`
  (returns (Return :type Boolean))
  (bind (_defaultworldrotation_roll _defaultworldrotation_pitch _defaultworldrotation_yaw) (`KismetMathLibrary.BreakRotator` (`self.DefaultWorldRotation`)))
  (bind (_returnvalue_roll _returnvalue_pitch _returnvalue_yaw) (`KismetMathLibrary.BreakRotator` (`SceneComponent.K2_GetComponentRotation` (`self.StaticMesh1`))))
  (return (select `bool` (> (`self.GetHorizontalDotProductTo` self (`GameplayStatics.GetPlayerCharacter` 0)) 0.0) :`false` (< _returnvalue_yaw _defaultworldrotation_yaw) :`true` (> _returnvalue_yaw _defaultworldrotation_yaw))))

(fn `UserConstructionScript`
  (`PrimitiveComponent.SetSimulatePhysics` (`self.StaticMesh1`) (`self.PhysicsInteraction?`)))